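; JarProjectile is a projectile Blueprint that damages characters whose tag differs from its owner's, then destroys itself.
; Tick counts down Lifetime and updates each attached modifier, destroying the actor on expiry.
; HitBox overlaps pass owner-scaled damage and weight to every modifier's OnHit before DoDamage, then spawn blood and shake the first player's camera.
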(event `self.ReceiveTick`
  (params (DeltaSeconds :type "Float (single-precision)"))
  (set `self.Lifetime` (- (`self.Lifetime`) DeltaSeconds))
  (if (<= (`self.Lifetime`) 0.0)
    (`self.K2_DestroyActor`)
    (else
      (for _array_element (`self.Modifiers`)
        (`/Game/Blueprints/Projectiles/ProjectileModifier.OnUpdate` _array_element DeltaSeconds)))))

(event `self.HitBox.OnComponentBeginOverlap`
  (params (OtherActor :type "Actor Object Reference") (OtherComp :type "PrimitiveComponent Object Reference") (OtherBodyIndex :type Integer) (bFromSweep :type Boolean) (SweepResult :type "EngineTypes.HitResult Structure (by ref)"))
  (bind _ownercharacter (`self.OwnerCharacter`))
  (bind _returnvalue (* (`self.Damage`) (`/Game/Blueprints/BaseCharacter.ProjectileDamageMultiplier` _ownercharacter)))
  (bind _returnvalue_2 (* (`self.Weight`) (`/Game/Blueprints/BaseCharacter.ProjectileWeightMultiplier` _ownercharacter)))
  (if (`KismetSystemLibrary.IsValid` (`self.OwnerCharacter`))
    (bind _asbasecharacter_c (cast `/Game/Blueprints/BaseCharacter` OtherActor))
    (if (not (`self.ActorHasTag` _asbasecharacter_c (`KismetArrayLibrary.Array_Get` (`Actor.Tags` (`self.OwnerCharacter`)))))
      (for _array_element (`self.Modifiers`)
        (`/Game/Blueprints/Projectiles/ProjectileModifier.OnHit` _array_element _asbasecharacter_c _returnvalue _returnvalue_2))
      (`/Game/Blueprints/BaseCharacter.DoDamage` _asbasecharacter_c _returnvalue _returnvalue_2 1.0)
      (`GameplayStatics.SpawnEmitterAtLocation` "/Game/Particles/Blood2.Blood2" (`self.K2_GetActorLocation` _asbasecharacter_c) (`KismetMathLibrary.Conv_VectorToRotator` (`KismetMathLibrary.GetRightVector` (`self.K2_GetActorRotation`))))
      (`PlayerController.ClientStartCameraShake` :`self` (`GameplayStatics.GetPlayerController` 0) :`Shake` "/Game/Blueprints/HitShake.HitShake_C" :`Scale` 15.0)
      (`self.K2_DestroyActor`))))

(fn `UserConstructionScript`
  (`parent.UserConstructionScript`))