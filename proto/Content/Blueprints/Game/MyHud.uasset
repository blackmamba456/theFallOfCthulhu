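; HUD class that draws character status labels, a kill counter and a top-right minimap on the canvas each frame.
; DrawHUD finds every living BaseCharacter and centers health, stamina and current-state text above its projected screen position.
; The minimap draws the player's SeenRooms as rectangles, adding strips in the wall gaps where sub-rooms have exits.
; The construction script caches the BP_LevelCreation actor, whose LevelSize anchors the minimap.
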(event `self.ReceiveDrawHUD`
  (params (SizeX :type Integer) (SizeY :type Integer))
  (bind _minimapcolor (`self.MinimapColor`))
  (bind _minimapwallscale (`self.MinimapWallScale`))
  (bind _minimapwallscale_2 (`self.MinimapWallScale`))
  (bind _x2 (`/Game/Blueprints/BP_Macros.F_x2` (`self.MinimapWallScale`)))
  (bind _returnvalue (- (`self.MinimapScale`) (`/Game/Blueprints/BP_Macros.F_x2` (`self.MinimapWallScale`))))
  (set `self.SizeX` SizeX)
  (set `self.SizeY` SizeY)
  (`|ExecutionSequence`
    (:`then_0`
      (bind _outactors (`GameplayStatics.GetAllActorsOfClass` "/Game/Blueprints/BaseCharacter.BaseCharacter_C"))
      (for _array_element _outactors
        (bind _asbasecharacter_c (cast `/Game/Blueprints/BaseCharacter` _array_element))
        (if (not (`/Game/Blueprints/BaseCharacter.Dead` _asbasecharacter_c))
          (`|ExecutionSequence`
            (:`then_0`
              (bind _returnvalue_2 (`KismetStringLibrary.Concat_StrStr` (`KismetStringLibrary.Concat_StrStr` (`KismetStringLibrary.Concat_StrStr` "Health: " (`KismetStringLibrary.Conv_DoubleToString` (`/Game/Blueprints/BaseCharacter.Health` _asbasecharacter_c))) "/") (`KismetStringLibrary.Conv_DoubleToString` (`/Game/Blueprints/BaseCharacter.MaxHealth` _asbasecharacter_c))))
              (bind _x (.x (`self.Project` (`self.K2_GetActorLocation` _asbasecharacter_c))))
              (bind _y (.y (`self.Project` (`self.K2_GetActorLocation` _asbasecharacter_c))))
              (`self.DrawText` _returnvalue_2 (struct :`R` 1.0 :`G` 1.0 :`B` 1.0 :`A` 1.0) (- _x (/ (`self.GetTextSize` _returnvalue_2 "/Game/Fonts/StandardFont.StandardFont" 1.0) 2.0)) (- _y 140.0) "/Game/Fonts/StandardFont.StandardFont" 1.0))
            (:`then_1`
              (bind _returnvalue_3 (`KismetStringLibrary.Concat_StrStr` (`KismetStringLibrary.Concat_StrStr` (`KismetStringLibrary.Concat_StrStr` "Stamina:  " (`KismetStringLibrary.Conv_DoubleToString` (`/Game/Blueprints/BaseCharacter.Stamina` _asbasecharacter_c))) "/") (`KismetStringLibrary.Conv_DoubleToString` (`/Game/Blueprints/BaseCharacter.MaxStamina` _asbasecharacter_c))))
              (`self.DrawText` _returnvalue_3 (struct :`R` 1.0 :`G` 1.0 :`B` 1.0 :`A` 1.0) (- _x (/ (`self.GetTextSize` _returnvalue_3 "/Game/Fonts/StandardFont.StandardFont" 1.0) 2.0)) (- _y 120.0) "/Game/Fonts/StandardFont.StandardFont" 1.0))
            (:`then_2`
              (bind _returnvalue_4 (`|GetEnumeratorNameAsString` (`/Game/Blueprints/BaseCharacter.CurrentState` _asbasecharacter_c)))
              (`self.DrawText` _returnvalue_4 (struct :`R` 1.0 :`G` 1.0 :`B` 1.0 :`A` 1.0) (- _x (/ (`self.GetTextSize` _returnvalue_4 "/Game/Fonts/StandardFont.StandardFont" 1.5) 2.0)) (- _y 100.0) "/Game/Fonts/StandardFont.StandardFont" 1.5))))))
    (:`then_1`
      (`self.DrawText` (`KismetStringLibrary.Concat_StrStr` "Kills: " (`KismetStringLibrary.Conv_IntToString` (`self.KillCount`))) (struct :`R` 1.0 :`G` 1.0 :`B` 1.0 :`A` 1.0) 10.0 10.0 "/Game/Fonts/StandardFont.StandardFont" 1.5))
    (:`then_2`
      ;[0 0 0] Minimap
      (set `self.MinimapPosition` (`KismetMathLibrary.MakeVector2D` (- (`KismetMathLibrary.Conv_IntToDouble` (`self.SizeX`)) (+ (* (`LevelCreation.levelSize` (`self.Level`)) (`self.MinimapScale`)) 10.0)) 10.0))
      (bind _asplayercharacter_c (cast `/Game/Blueprints/PlayerCharacter` (`GameplayStatics.GetPlayerPawn` 0)))
      (for _array_element_2 (`/Game/Blueprints/PlayerCharacter.seenRooms` _asplayercharacter_c)
        (`|ExecutionSequence`
          (:`then_0`
            (bind (_x_2 _y_2) (`KismetMathLibrary.BreakVector2D` (+ (* (`IRoom.position` _array_element_2) (`self.MinimapScale`)) (`self.MinimapPosition`))))
            (`self.DrawRect` (`self.MinimapColor`) (+ _x_2 _minimapwallscale_2) (+ _y_2 _minimapwallscale_2) (- (* (`IRoom.width` _array_element_2) (`self.MinimapScale`)) _x2) (- (* (`IRoom.height` _array_element_2) (`self.MinimapScale`)) _x2)))
          (:`then_1`
            (for _index (range (`IRoom.height` _array_element_2))
              (bind _width (`IRoom.width` _array_element_2))
              (for _index_2 (range _width)
                (`|ExecutionSequence`
                  (:`then_0`
                    (bind (_exitleft _exitright _exitup _exitdown) (break `IRoom.SubRoom` (`KismetArrayLibrary.Array_Get` (`IRoom.subRooms` _array_element_2) (+ _index_2 (* _index _width)))))
                    (if _exitleft
                      (bind (_x_3 _y_3) (`KismetMathLibrary.BreakVector2D` (+ (* (`IRoom.position` _array_element_2) (`self.MinimapScale`)) (`self.MinimapPosition`))))
                      (bind _returnvalue_5 (+ _x_3 (* _index_2 (`self.MinimapScale`))))
                      (bind _returnvalue_6 (+ _y_3 (* _index (`self.MinimapScale`))))
                      (bind _returnvalue_7 (+ _returnvalue_6 (`self.MinimapWallScale`)))
                      (`self.DrawRect` _minimapcolor _returnvalue_5 _returnvalue_7 _minimapwallscale _returnvalue)))
                  (:`then_1`
                    (if _exitright
                      (`self.DrawRect` _minimapcolor (+ _returnvalue_5 (- (`self.MinimapScale`) (`self.MinimapWallScale`))) _returnvalue_7 _minimapwallscale _returnvalue)))
                  (:`then_2`
                    (if _exitup
                      (bind _returnvalue_8 (+ _returnvalue_5 (`self.MinimapWallScale`)))
                      (`self.DrawRect` _minimapcolor _returnvalue_8 _returnvalue_6 _returnvalue _minimapwallscale)))
                  (:`then_3`
                    (if _exitdown
                      (`self.DrawRect` _minimapcolor _returnvalue_8 (+ _returnvalue_6 (- (`self.MinimapScale`) (`self.MinimapWallScale`))) _returnvalue _minimapwallscale))))))))))))

(fn `UserConstructionScript`
  (bind _outactors (`GameplayStatics.GetAllActorsOfClass` "/Game/Blueprints/BP_LevelCreation.BP_LevelCreation_C"))
  (bind _asbp_levelcreation_c (cast `/Game/Blueprints/BP_LevelCreation` (`KismetArrayLibrary.Array_Get` _outactors)))
  (set `self.Level` _asbp_levelcreation_c))