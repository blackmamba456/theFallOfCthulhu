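; EnemyCharacter is an enemy character Blueprint that arms itself with a weapon and shield and can block.
; On BeginPlay it spawns and equips a BaseWeapon and a left-hand Shield, then calls Initialize.
; StartBlock activates the left-hand item unless it is already active or the character is in one particular state, and EndBlock deactivates it.
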(event `self.ReceiveBeginPlay`
  (`|ExecutionSequence`
    (:`then_0`
      (bind _returnvalue (`|SpawnActorFromClass` "/Game/Blueprints/Items/BaseWeapon.BaseWeapon_C" (`KismetMathLibrary.MakeTransform` (0.0 0.0 0.0)) true))
      (`self.EquipWeapon` _returnvalue))
    (:`then_1`
      (bind _returnvalue_2 (`|SpawnActorFromClass` "/Game/Blueprints/Items/Shield.Shield_C" (`KismetMathLibrary.MakeTransform` (0.0 0.0 0.0)) true))
      (`self.EquipLeftHandItem` _returnvalue_2))
    (:`then_2`
      (`self.Initialize`))))

(event `StartBlock`
  (if (and (not (`|EnumEquality` (`self.CurrentState`) "NewEnumerator2")) (not (`/Game/Blueprints/Items/BaseItem.Active` (`self.LeftHandItem`))))
    (`self.ActivateLeftHandItemEvent`)))

(event `EndBlock`
  (`self.DeactivateLeftHandItemEvent`))

(fn `UserConstructionScript`
  (`parent.UserConstructionScript`))