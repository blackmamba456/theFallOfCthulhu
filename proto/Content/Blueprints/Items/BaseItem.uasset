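; BaseItem is a base item Blueprint with an active state, a cooldown and empty gameplay hooks.
; UpdateEvent counts the cooldown down each call and runs ActiveTick while the item is active.
; Activate and Deactivate toggle the active state and fire their events, with activation gated by the cooldown, which neither function resets.
; Empty events cover attacks, hits dealt and received, rolls, jumps and passive application.
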(event `UpdateEvent`
  (params (`Delta Seconds` :type "Float (double-precision)"))
  (set `self.Cooldown` (- (`self.Cooldown`) `Delta Seconds`))
  (if (`self.Active`)
    (`self.ActiveTick` `Delta Seconds`)))

(event `OnAttack`)

(event `OnActivate`)

(event `ActiveTick`
  (params (`Delta Secconds` :type "Float (double-precision)")))

(event `OnDeactivate`)

(event `OnHit`
  (params (HitCharacter :type "/Game/Blueprints/BaseCharacter Object Reference") (AttackDamage :type "Float (double-precision)") (AttackWeight :type "Float (double-precision)")))

(event `OnReceivedHit`
  (params (OtherCharacter :type "/Game/Blueprints/BaseCharacter Object Reference") (AttackDamage :type "Float (double-precision)") (AttackWeight :type "Float (double-precision)")))

(event `OnRoll`)

(event `OnJump`)

(event `OnApplyPassives`)

(event `OnSuccessfulHit`
  (params (HitCharacter :type "/Game/Blueprints/BaseCharacter Object Reference") (AttackDamage :type "Float (double-precision)") (AttackWeight :type "Float (double-precision)")))

(event `OnUnsuccessfulHit`
  (params (HitCharacter :type "/Game/Blueprints/BaseCharacter Object Reference") (AttackDamage :type "Float (double-precision)") (AttackWeight :type "Float (double-precision)")))

(fn `Activate`
  (if (<= (`self.Cooldown`) 0.0)
    (if (not (`self.Active`))
      (set `self.Active` true)
      (`self.OnActivate`))))

(fn `Deactivate`
  (if (`self.Active`)
    (set `self.Active` false)
    (`self.OnDeactivate`)))

(fn `UserConstructionScript`)