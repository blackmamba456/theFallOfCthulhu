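; BP_Pickup is a world pickup that gives a player character an item of a configurable ItemClass.
; When the Action input is pressed, it runs a box overlap query over its Trigger volume for PlayerCharacter pawns.
; For an overlapping character, it spawns the item at the world origin, adds it to that character's Items, sets its UserCharacter and destroys itself.
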(event `InputAction|Action`
  (bind _trigger (`self.Trigger`))
  (:`Pressed`
    (bind _outactors (`KismetSystemLibrary.BoxOverlapActors_NEW` (`SceneComponent.K2_GetComponentLocation` _trigger) (`BoxComponent.GetScaledBoxExtent` _trigger) (`|MakeArray` "ObjectTypeQuery3" :!type "EngineTypes.EObjectTypeQuery Enum") "/Game/Blueprints/PlayerCharacter.PlayerCharacter_C"))
    (for _array_element _outactors
      (bind _asplayercharacter_c (cast `/Game/Blueprints/PlayerCharacter` _array_element))
      (bind _returnvalue (`|SpawnActorFromClass` (`self.ItemClass`) (`KismetMathLibrary.MakeTransform` (0.0 0.0 0.0))))
      (bind _asbaseitem_c (cast `/Game/Blueprints/Items/BaseItem` _returnvalue))
      (`KismetArrayLibrary.Array_Add` (`/Game/Blueprints/BaseCharacter.Items` _asplayercharacter_c) _asbaseitem_c)
      (set `/Game/Blueprints/Items/BaseItem.UserCharacter` _asplayercharacter_c _asbaseitem_c)
      (`self.K2_DestroyActor`))))

(fn `UserConstructionScript`)