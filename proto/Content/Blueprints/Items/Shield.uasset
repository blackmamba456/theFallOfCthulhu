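; Shield item that lets its user block frontal hits at the cost of stamina.
; While active it cuts the user's stamina recovery and movement speed, restoring both on deactivation, and it drops when stamina is empty.
; A forward-vector dot product detects facing attackers, whose attack weight drains stamina.
; A successful block repels and invalidates the attack, while a broken guard repels the user and scales damage by the stamina shortfall.
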(event `self.OnActivate`
  (bind _usercharacter (`self.UserCharacter`))
  (set `/Game/Blueprints/BaseCharacter.StaminaRecovery` (* (`/Game/Blueprints/BaseCharacter.StaminaRecovery` _usercharacter) 0.1) _usercharacter)
  (set `/Game/Blueprints/BaseCharacter.MovementSpeed` (* (`/Game/Blueprints/BaseCharacter.MovementSpeed` _usercharacter) 0.5) _usercharacter)
  (if (<= (`/Game/Blueprints/BaseCharacter.Stamina` _usercharacter) 0.0)
    (`self.Deactivate`)))

(event `self.OnDeactivate`
  (bind _usercharacter (`self.UserCharacter`))
  (set `/Game/Blueprints/BaseCharacter.StaminaRecovery` (/ (`/Game/Blueprints/BaseCharacter.StaminaRecovery` _usercharacter) 0.1) _usercharacter)
  (set `/Game/Blueprints/BaseCharacter.MovementSpeed` (/ (`/Game/Blueprints/BaseCharacter.MovementSpeed` _usercharacter) 0.5) _usercharacter))

(event `self.OnReceivedHit`
  (params (OtherCharacter :type "/Game/Blueprints/BaseCharacter Object Reference") (AttackDamage :type "Float (single-precision)") (AttackWeight :type "Float (single-precision)"))
  (bind _usercharacter (`self.UserCharacter`))
  (bind _stamina (`/Game/Blueprints/BaseCharacter.Stamina` _usercharacter))
  (if (`self.Active`)
    (if (< (`KismetMathLibrary.Dot_VectorVector` (`KismetMathLibrary.GetForwardVector` (`self.K2_GetActorRotation` (`self.UserCharacter`))) (`KismetMathLibrary.GetForwardVector` (`self.K2_GetActorRotation` OtherCharacter))) 0.0)
      (set `/Game/Blueprints/BaseCharacter.Stamina` (- (`/Game/Blueprints/BaseCharacter.Stamina` _usercharacter) AttackWeight) _usercharacter)
      (if (<= _stamina 0.0)
        (`self.Deactivate`)
        (`/Game/Blueprints/BaseCharacter.Repell` _usercharacter)
        (set `/Game/Blueprints/BaseCharacter.DamagePercentage` (* (/ (* _stamina -1.0) AttackWeight) AttackDamage) _usercharacter)
        (else
          (`/Game/Blueprints/BaseCharacter.Repell` OtherCharacter)
          (`/Game/Blueprints/BaseCharacter.InvalidateHit` OtherCharacter)
          (set `/Game/Blueprints/BaseCharacter.DamagePercentage` 0.0 OtherCharacter))))))

(fn `UserConstructionScript`
  (`parent.UserConstructionScript`))