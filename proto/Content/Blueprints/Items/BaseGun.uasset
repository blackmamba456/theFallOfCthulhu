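; BaseGun is a gun item that, when activated, fires a default BaseProjectile, sets its cooldown and deactivates.
; SpawnProjectile passes owner, damage, weight, lifetime and modifiers to the spawned projectile, then calls OnCreate on each modifier.
; Zero position or direction inputs trigger defaults: the gun's location with the user's Y, and velocity along world ±Y chosen by the user's facing.
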(event `self.OnActivate`
  (`self.SpawnProjectile` "/Game/Blueprints/Projectiles/BaseProjectile.BaseProjectile_C" (0.0 0.0 0.0) (0.0 0.0 0.0) 2000.0 10.0 51.0 3.0 (`|MakeArray`))
  (set `self.Cooldown` 1.0)
  (`self.Deactivate`))

(fn `SpawnProjectile`
  (params (ProjectileClass :type "/Game/Blueprints/Projectiles/BaseProjectile Class Reference") (Position :type "Object.Vector Structure") (Direction :type "Object.Vector Structure") (Speed :type "Float (double-precision)") (Damage :type "Float (double-precision)") (Weight :type "Float (double-precision)") (Lifetime :type "Float (double-precision)") (Modifiers :type "Array of /Game/Blueprints/Projectiles/ProjectileModifier Object Reference"))
  (bind _returnvalue (`|SpawnActorFromClass` ProjectileClass (`KismetMathLibrary.MakeTransform` (`KismetMathLibrary.SelectVector` (`KismetMathLibrary.MakeVector` (.x (`self.K2_GetActorLocation`)) (.y (`self.K2_GetActorLocation` (`self.UserCharacter`))) (.z (`self.K2_GetActorLocation`))) Position (== Position (0.0 0.0 0.0)))) true))
  (bind _asbaseprojectile_c (cast `/Game/Blueprints/Projectiles/BaseProjectile` _returnvalue))
  (set `MovementComponent.Velocity` (* (`KismetMathLibrary.SelectVector` (`KismetMathLibrary.SelectVector` (0.0 1.0 0.0) (0.0 -1.0 0.0) (> (`KismetMathLibrary.Dot_VectorVector` (`KismetMathLibrary.GetForwardVector` (`self.K2_GetActorRotation` (`self.UserCharacter`))) (0.0 1.0 0.0)) 0.0)) Direction (== Direction (0.0 0.0 0.0))) Speed) (`/Game/Blueprints/Projectiles/BaseProjectile.ProjectileMovement` _asbaseprojectile_c))
  (set `/Game/Blueprints/Projectiles/BaseProjectile.OwnerCharacter` (`self.UserCharacter`) _asbaseprojectile_c)
  (set `/Game/Blueprints/Projectiles/BaseProjectile.Damage` Damage _asbaseprojectile_c)
  (set `/Game/Blueprints/Projectiles/BaseProjectile.Weight` Weight _asbaseprojectile_c)
  (set `/Game/Blueprints/Projectiles/BaseProjectile.Lifetime` Lifetime _asbaseprojectile_c)
  (set `/Game/Blueprints/Projectiles/BaseProjectile.Modifiers` Modifiers _asbaseprojectile_c)
  (for _array_element (`/Game/Blueprints/Projectiles/BaseProjectile.Modifiers` _asbaseprojectile_c)
    (`/Game/Blueprints/Projectiles/ProjectileModifier.OnCreate` _array_element)))

(fn `UserConstructionScript`
  (`parent.UserConstructionScript`))