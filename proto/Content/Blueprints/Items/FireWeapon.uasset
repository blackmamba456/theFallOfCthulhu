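; FireWeapon is a two-handed weapon item that sets the struck character on fire, draining its health over time.
; A successful hit spawns a fire emitter on the victim, replacing any previous one, resets the burn timer and activates the item.
; While active, its tick applies burn damage and moves the flame with the victim until the timer expires or the victim dies, then removes it and deactivates.
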(event `self.ReceiveBeginPlay`
  (`StaticMeshComponent.SetStaticMesh` (`self.Mesh`) "/Game/StaticMeshes/weapons/twoHanded.twoHanded"))

(event `self.OnSuccessfulHit`
  (params (HitCharacter :type "/Game/Blueprints/BaseCharacter Object Reference") (AttackDamage :type "Float (single-precision)") (AttackWeight :type "Float (single-precision)"))
  (bind _enemyfireeffect (`self.EnemyFireEffect`))
  (set `self.HitChar` HitCharacter)
  (bind _returnvalue (`GameplayStatics.SpawnEmitterAtLocation` "/Game/Particles/Fire.Fire" (`self.K2_GetActorLocation` HitCharacter)))
  (if (`KismetSystemLibrary.IsValid` _enemyfireeffect)
    (`ActorComponent.K2_DestroyComponent` _enemyfireeffect))
  (set `self.EnemyFireEffect` _returnvalue)
  (set `self.BurnTime` 5.0)
  (`self.Activate`))

(event `self.ActiveTick`
  (params (`Delta Secconds` :type "Float (single-precision)"))
  (bind _hitchar (`self.HitChar`))
  (set `self.BurnTime` (- (`self.BurnTime`) `Delta Secconds`))
  (if (or (<= (`self.BurnTime`) 0.0) (`/Game/Blueprints/BaseCharacter.Dead` (`self.HitChar`)))
    (`ActorComponent.K2_DestroyComponent` (`self.EnemyFireEffect`))
    (`self.Deactivate`)
    (else
      (set `/Game/Blueprints/BaseCharacter.Health` (- (`/Game/Blueprints/BaseCharacter.Health` _hitchar) (* 2.0 `Delta Secconds`)) _hitchar)
      (`SceneComponent.SetWorldLocation` (`self.EnemyFireEffect`) (`self.K2_GetActorLocation` _hitchar) false))))

(fn `UserConstructionScript`
  (`parent.UserConstructionScript`))