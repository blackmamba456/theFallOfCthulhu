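; BP_EnemySpawner is a placeable spawner that may spawn one AI enemy at its own location and rotation when play begins.
; It reads the current Level from BP_GameInstance, samples the SpawnChance curve at that level, and rolls a random percentage against the result.
; A successful roll spawns EnemyCharacter with EnemyBehaviourTree, ignoring collision so the spawn is not blocked.
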(event `self.ReceiveBeginPlay`
  (bind _asbp_gameinstance_c (cast `/Game/Blueprints/Game/BP_GameInstance` (`GameplayStatics.GetGameInstance`)))
  (if (<= (`KismetMathLibrary.RandomFloatInRange` 0.0 100.0) (`CurveFloat.GetFloatValue` (`self.SpawnChance`) (`KismetMathLibrary.Conv_IntToDouble` (`/Game/Blueprints/Game/BP_GameInstance.Level` _asbp_gameinstance_c))))
    (`AIBlueprintHelperLibrary.SpawnAIFromClass` "/Game/Blueprints/Enemies/EnemyCharacter.EnemyCharacter_C" "/Game/Blueprints/Enemies/AI/EnemyBehaviourTree.EnemyBehaviourTree" (.location (`self.GetTransform`)) (.rotation (`self.GetTransform`)) true)))

(fn `UserConstructionScript`)