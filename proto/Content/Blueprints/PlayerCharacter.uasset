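; Player-controlled character Blueprint that spawns with a base weapon and a shield.
; On BeginPlay it spawns and equips both items, then runs initialization, and Tick forwards delta time to an update event.
; Input axis and actions for movement, roll, jump, light and strong attacks, left-hand item and action are relayed to event functions or a dispatcher.
; Roll and attacks also receive the current MoveRight value.
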(event `self.ReceiveBeginPlay`
  (bind _returnvalue (`|SpawnActorFromClass` "/Game/Blueprints/Items/BaseWeapon.BaseWeapon_C" (`KismetMathLibrary.MakeTransform` (0.0 0.0 0.0)) true))
  (`self.EquipWeapon` _returnvalue)
  (bind _returnvalue_2 (`|SpawnActorFromClass` "/Game/Blueprints/Items/Shield.Shield_C" (`KismetMathLibrary.MakeTransform` (0.0 0.0 0.0)) true))
  (`self.EquipLeftHandItem` _returnvalue_2)
  (`self.Initialize`))

(event `self.ReceiveTick`
  (params (DeltaSeconds :type "Float (single-precision)"))
  (`self.UpdateEvent` DeltaSeconds))

(event `InputAxis|MoveRight`
  (params (AxisValue :type "Float (single-precision)"))
  (`self.MoveEvent` AxisValue))

(event `InputAction|Roll`
  (:`Pressed`
    (`self.RollEvent` (`self.GetInputAxisValue`))))

(event `InputAction|Jump`
  (:`Pressed`
    (`self.JumpEvent`)))

(event `InputAction|LeftHandItem`
  (:`Pressed`
    (`self.ActivateLeftHandItemEvent`))
  (:`Released`
    (`self.DeactivateLeftHandItemEvent`)))

(event `InputAction|Light Attack`
  (:`Pressed`
    (`self.LightAttackEvent` (`self.GetInputAxisValue`))))

(event `InputAction|Strong Attack`
  (:`Pressed`
    (`self.StrongAttackEvent` (`self.GetInputAxisValue`))))

(event `InputAction|Action`
  (:`Pressed`
    (`self.ActionDispatcher`)))

(fn `UserConstructionScript`
  (`parent.UserConstructionScript`))