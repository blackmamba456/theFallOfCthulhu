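; Base heal room Blueprint that restores the player character's health while the player pawn overlaps it.
; Begin and end overlap events for player pawn 0 open and close a Gate on Tick.
; While the gate is open, each tick adds HealRate scaled by delta time to the PlayerCharacter's Health, capped at MaxHealth.
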(event `self.ReceiveTick`
  (params (DeltaSeconds :type "Float (single-precision)"))
  (`/Engine/EditorBlueprintResources/StandardMacros.Gate` true :!label _label
    (:`Exit`
      (bind _asplayercharacter_c (cast `/Game/Blueprints/PlayerCharacter` (`GameplayStatics.GetPlayerPawn` 0)))
      (set `/Game/Blueprints/BaseCharacter.Health` (`KismetMathLibrary.FMin` (+ (* DeltaSeconds (`self.healRate`)) (`/Game/Blueprints/BaseCharacter.Health` _asplayercharacter_c)) (`/Game/Blueprints/BaseCharacter.MaxHealth` _asplayercharacter_c)) _asplayercharacter_c))))

(event `self.ReceiveActorBeginOverlap`
  (params (OtherActor :type "Actor Object Reference"))
  (if (== (`GameplayStatics.GetPlayerPawn` 0) OtherActor)
    (goto _label :!via `Open`)))

(event `self.ReceiveActorEndOverlap`
  (params (OtherActor :type "Actor Object Reference"))
  (if (== (`GameplayStatics.GetPlayerPawn` 0) OtherActor)
    (goto _label :!via `Close`)))

(fn `UserConstructionScript`
  (`parent.UserConstructionScript`))