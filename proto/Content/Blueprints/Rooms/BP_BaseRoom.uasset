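; BP_BaseRoom is a base room actor that shows or hides its contents as a group.
; Actors that begin overlapping it, except those of class IRoom, join ContainedActors and immediately match the room's Visible state.
; SetVisibility stores the state and applies it to contained actors and Walls, while always keeping the room actor itself unhidden.
; The removal on end overlap is disconnected, so actors stay in the list after leaving.
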(event `self.ReceiveActorBeginOverlap`
  (params (OtherActor :type "Actor Object Reference"))
  (if (!= (`GameplayStatics.GetObjectClass` OtherActor) "/Script/proto.IRoom")
    (bind _returnvalue (`KismetArrayLibrary.Array_Add` (`self.ContainedActors`) OtherActor))
    (`self.SetActorHiddenInGame` (`KismetArrayLibrary.Array_Get` (`self.ContainedActors`) _returnvalue) (not (`self.visible`)))))

(event `self.ReceiveActorEndOverlap`
  (params (OtherActor :type "Actor Object Reference"))
  (if (!= (`GameplayStatics.GetObjectClass` OtherActor) "/Script/proto.IRoom")
    _))

(fn `setVisibility`
  (params (visibility :type Boolean))
  (bind _returnvalue (not visibility))
  (set `self.visible` visibility)
  (for _array_element (`self.ContainedActors`)
    (`self.SetActorHiddenInGame` _array_element _returnvalue))
  (for _array_element_2 (`self.walls`)
    (`self.SetActorHiddenInGame` _array_element_2 _returnvalue))
  (`self.SetActorHiddenInGame` false))

(fn `UserConstructionScript`)