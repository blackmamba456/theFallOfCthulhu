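; BP_GUIPage is an actor that wraps one menu page widget in the HUD's GUI navigation.
; Its construction script creates the widget from WidgetClass as a BasePage, and events add it to or remove it from the viewport, including removal on EndPlay.
; The widget's back dispatcher is forwarded to Manager.Back.
; SwitchToLastPage swaps to LastPage when valid and returns the active page, otherwise itself.
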(event Custom|AddToViewport
  (UserInterface|Viewport|AddtoViewport (Variables|Default|Getwidget)))

(event Custom|RemoveFromViewPort
  (Class|UserWidget|RemovefromViewport (Variables|Default|Getwidget)))

(event Custom|Back
  (Default|Back (Variables|Default|Getmanager)))

(event EventEndPlay
  (params (EndPlayReason :type EEndPlayReason%20Enum :default "ActorDestroyed"))
  (Class|UserWidget|RemovefromViewport (Variables|Default|Getwidget)))

(event EventBeginPlay
  (EventDispatchers|BindEventtoBackDispatcher (Variables|Default|Getwidget) (delegate Custom|Back)))

(fn ConstructionScript
  (bind _returnvalue (UserInterface|CreateWidget (Variables|Default|GetwidgetClass)))
  (bind _asbasepage_c (Utilities|Casting|CastToBasePage _returnvalue))
  (Variables|Default|Setwidget _asbasepage_c))

(fn SwitchtoLastPage
  (if (Utilities|IsValid (Variables|Default|GetlastPage))
    (Class|UserWidget|RemovefromViewport (Variables|Default|Getwidget))
    (CallFunction|AddtoViewport (Variables|Default|GetlastPage))
    (LocalVariables|Setreturn (Variables|Default|GetlastPage))
    (else
      (LocalVariables|Setreturn self)))
  (return (LocalVariables|Getreturn)))