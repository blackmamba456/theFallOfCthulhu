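; BP_OptionsPage builds and routes the options section of the menu, covering video and audio settings.
; On BeginPlay it spawns BP_GUIPage actors for the options, graphics and sound menus, with both submenus using the options page as their LastPage.
; Options widget dispatchers trigger Manager.SwitchMenu to the matching page, and SwitchToOptionMenu opens the options page.
; The sound widget receives a newly spawned SoundConfigs actor.
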(event `self.ReceiveBeginPlay`
  (bind _returnvalue (`KismetMathLibrary.MakeTransform` (0.0 0.0 0.0)))
  (bind _manager (`self.manager`))
  (`|ExecutionSequence`
    (:`then_0`
      (bind _returnvalue_2 (`|SpawnActorFromClass` "/Game/Blueprints/HUD/menu/BP_GUIPage.BP_GUIPage_C" _returnvalue false (`self.lastPage`) "/Game/Blueprints/HUD/menu/OptionsMenu.OptionsMenu_C" _manager))
      (set `self.optionMenu` _returnvalue_2)
      (bind _asoptionsmenu_c (cast `/Game/Blueprints/HUD/menu/OptionsMenu` (`/Game/Blueprints/HUD/menu/BP_GUIPage.widget` (`self.optionMenu`))))
      (`|ExecutionSequence`
        (:`then_0`
          (add `/Game/Blueprints/HUD/menu/OptionsMenu.VideoDispatcher` _asoptionsmenu_c (delegate `Video`)))
        (:`then_1`
          (add `/Game/Blueprints/HUD/menu/OptionsMenu.AudioDispatcher` _asoptionsmenu_c (delegate `Audio`)))))
    (:`then_1`
      (bind _returnvalue_3 (`|SpawnActorFromClass` "/Game/Blueprints/HUD/menu/BP_GUIPage.BP_GUIPage_C" _returnvalue false (`self.optionMenu`) "/Game/Blueprints/HUD/menu/GraphicsSettingsMenu.GraphicsSettingsMenu_C" _manager))
      (set `self.videoMenu` _returnvalue_3))
    (:`then_2`
      (bind _returnvalue_4 (`|SpawnActorFromClass` "/Game/Blueprints/HUD/menu/BP_GUIPage.BP_GUIPage_C" _returnvalue false (`self.optionMenu`) "/Game/Blueprints/HUD/menu/SoundSettingsMenu.SoundSettingsMenu_C" _manager))
      (set `self.audioMenu` _returnvalue_4)
      (bind _assoundsettingsmenu_c (cast `/Game/Blueprints/HUD/menu/SoundSettingsMenu` (`/Game/Blueprints/HUD/menu/BP_GUIPage.widget` (`self.audioMenu`))))
      (bind _returnvalue_5 (`|SpawnActorFromClass` "/Script/proto.SoundConfigs" (`KismetMathLibrary.MakeTransform` (0.0 0.0 0.0) (struct) (1.0 1.0 1.0))))
      (`/Game/Blueprints/HUD/menu/SoundSettingsMenu.SetConfig` _assoundsettingsmenu_c _returnvalue_5))))

(event `Video`
  (`/Game/Blueprints/HUD/menu/BP_PageManager.switchMenu` (`self.manager`) (`self.videoMenu`)))

(event `Audio`
  (`/Game/Blueprints/HUD/menu/BP_PageManager.switchMenu` (`self.manager`) (`self.audioMenu`)))

(event `SwitchToOptionMenu`
  (`/Game/Blueprints/HUD/menu/BP_PageManager.switchMenu` (`self.manager`) (`self.optionMenu`)))

(fn `UserConstructionScript`)