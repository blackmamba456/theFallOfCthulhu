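; HUD that draws kill count, state text over living characters, a fading player stamina bar and a four-point inventory around the player.
; DrawHUD also drives player camera vignette from health and shortens the spring arm while the inventory is open.
; Inventory markers fade by mouse direction and distance from the player.
; Only the left slot has a hitbox-driven scrollable icon grid, filled with test items linked by name prefix.
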(event EventDrawHUD
  (params (SizeX :type Integer) (SizeY :type Integer))
  (bind _inventorypositions (Variables|Default|GetInventoryPositions))
  (bind _item (Utilities|Array|Get(acopy) _inventorypositions))
  (bind _item_2 (Utilities|Array|Get(acopy) _inventorypositions 3))
  (bind _item_3 (Utilities|Array|Get(acopy) _inventorypositions 1))
  (bind _item_4 (Utilities|Array|Get(acopy) _inventorypositions 2))
  (bind (_x _y) (Math|Vector2D|BreakVector2D _item))
  (bind (_x_2 _y_2) (Math|Vector2D|BreakVector2D _item_2))
  (bind (_x_3 _y_3) (Math|Vector2D|BreakVector2D _item_3))
  (bind (_x_4 _y_4) (Math|Vector2D|BreakVector2D _item_4))
  (Utilities|FlowControl|Sequence
    (:then_0
      ;[1 1 1] Calculate HUD Fade
      (if (> (Variables|Default|GetFadeCounter) 0.0)
        (Variables|Default|SetFadeCounter (- (Variables|Default|GetFadeCounter) (Utilities|Time|GetWorldDeltaSeconds)))
        (Variables|Default|SetHudFade (Math|Float|Clamp(Float) (+ (Variables|Default|GetHudFade) 0.05) 0.0 0.8))
        (else
          (Variables|Default|SetHudFade (Math|Float|Clamp(Float) (- (Variables|Default|GetHudFade) 0.01) 0.0 0.8)))))
    (:then_1
      (bind _outactors (Actor|GetAllActorsOfClass "/Game/Blueprints/BaseCharacter.BaseCharacter_C"))
      (for _array_element _outactors
        (bind _asbasecharacter_c (Utilities|Casting|CastToBaseCharacter _array_element))
        (if (not (Variables|/Game/Blueprints/BaseCharacter.BaseCharacter_C|GetDead _asbasecharacter_c))
          (Utilities|FlowControl|Sequence
            (:then_0
              (if (Utilities|Name|Equal(Name) (Utilities|Array|Get(acopy) (Variables|/Script/Engine.Actor|GetTags _asbasecharacter_c)) "Player")
                (if (and (> (Variables|/Game/Blueprints/BaseCharacter.BaseCharacter_C|GetStamina _asbasecharacter_c) 0.0) (< (Variables|/Game/Blueprints/BaseCharacter.BaseCharacter_C|GetStamina _asbasecharacter_c) (Variables|/Game/Blueprints/BaseCharacter.BaseCharacter_C|GetMaxStamina _asbasecharacter_c)))
                  (Variables|Default|SetFadeCounter 1.0)
                  (Canvas|DrawTexture "/Game/Materials/textures/StaminaBar.StaminaBar" (- (.X (Math|Vector|BreakVector (Class|HUD|Project (Transformation|GetActorLocation _asbasecharacter_c)))) 128.0) (+ (.Y (Math|Vector|BreakVector (Class|HUD|Project (Transformation|GetActorLocation _asbasecharacter_c)))) 1.5e+02) (* (/ (Variables|/Game/Blueprints/BaseCharacter.BaseCharacter_C|GetStamina _asbasecharacter_c) (Variables|/Game/Blueprints/BaseCharacter.BaseCharacter_C|GetMaxStamina _asbasecharacter_c)) 256.0) 64.0 0.0 0.0 (/ (Variables|/Game/Blueprints/BaseCharacter.BaseCharacter_C|GetStamina _asbasecharacter_c) (Variables|/Game/Blueprints/BaseCharacter.BaseCharacter_C|GetMaxStamina _asbasecharacter_c)) 1.0 (Math|Color|MakeColor 1.0 1.0 1.0 (Variables|Default|GetHudFade)) :!label _label)
                  (elif (> (Variables|/Game/Blueprints/BaseCharacter.BaseCharacter_C|GetStamina _asbasecharacter_c) 0.0)
                    (goto _label)))))
            (:then_1
              (HUD|DrawText (Utilities|String|EnumtoString (Variables|/Game/Blueprints/BaseCharacter.BaseCharacter_C|GetCurrentState _asbasecharacter_c)) "(R=1.000000,G=1.000000,B=1.000000,A=1.000000)" (- (.X (Math|Vector|BreakVector (Class|HUD|Project (Transformation|GetActorLocation _asbasecharacter_c)))) (/ (.OutWidth (Class|HUD|GetTextSize (Utilities|String|EnumtoString (Variables|/Game/Blueprints/BaseCharacter.BaseCharacter_C|GetCurrentState _asbasecharacter_c)) "/Game/Fonts/StandardFont.StandardFont" 1.5)) 2.0)) (- (.Y (Math|Vector|BreakVector (Class|HUD|Project (Transformation|GetActorLocation _asbasecharacter_c)))) 1.5e+02) "/Game/Fonts/StandardFont.StandardFont" 1.5 false))
            (:then_2
              (bind _asplayercharacter_c (Utilities|Casting|CastToPlayerCharacter _asbasecharacter_c))
              (Variables|/Script/Engine.CameraComponent|SetPostProcessSettings (Variables|/Game/Blueprints/PlayerCharacter.PlayerCharacter_C|GetCamera1 _asplayercharacter_c) (Utilities|Struct|MakePostProcessSettings false false false false false false false false false false false false false false false false false false false false false false false false false false false false false false false false false false false false false false false false false false false false false false false true true false false false false false false false false false false false false false false false false false false false false false false false false false false false false false false false false false false false false false false false false false false false false false false false false false false false "(R=1.000000,G=1.000000,B=1.000000,A=1.000000)" "(R=1.000000,G=1.000000,B=1.000000,A=1.000000)" 0.5 0.0 1.0 "(R=1.000000,G=0.000000,B=0.000000,A=1.000000)" "(R=0.000000,G=1.000000,B=0.000000,A=1.000000)" "(R=0.000000,G=0.000000,B=1.000000,A=1.000000)" 0.03 1.0 0.18 4.0 "(R=1.000000,G=1.000000,B=1.000000,A=1.000000)" 0.0 0.5 1.0 1.0 1.0 4.0 16.0 32.0 1e+02 "(R=0.500000,G=0.500000,B=0.500000,A=1.000000)" "(R=0.500000,G=0.500000,B=0.500000,A=1.000000)" "(R=0.500000,G=0.500000,B=0.500000,A=1.000000)" "(R=0.500000,G=0.500000,B=0.500000,A=1.000000)" "(R=0.500000,G=0.500000,B=0.500000,A=1.000000)" 1.0 "(R=0.500000,G=0.500000,B=0.500000,A=1.000000)" 0 1.0 0.0 0.64 5312.0 0.0 0.0 0.384 1.0 1.0 "(R=1.000000,G=1.000000,B=1.000000,A=1.000000)" 1.0 0 8e+01 98.300003 0.03 2.0 3.0 1.0 0.0 -8.0 4.0 1.0 "(R=1.000000,G=1.000000,B=1.000000,A=1.000000)" 3.0 8.0 0 (- 1.5 (* (/ (Variables|/Game/Blueprints/BaseCharacter.BaseCharacter_C|GetHealth _asplayercharacter_c) (Variables|/Game/Blueprints/BaseCharacter.BaseCharacter_C|GetMaxHealth _asplayercharacter_c)) 1.5)) "(R=0.025000,G=0.000000,B=0.000000,A=1.000000)" 0.0 0.0 0.5 1.0 4e+01 false 8e+03 5e+03 8e+01 2.0 3.0 5e+01 0.6 1.7 0.01 "(R=1.000000,G=1.000000,B=1.000000,A=1.000000)" 1.0 1.0 0 "DOFM_BokehDOF" 1e+03 0.0 3e+02 5e+02 0.0 15.0 15.0 15.0 0 0.4 1.0 0.08 0.0 0.5 5.0 0.5 1e+02 "AAM_TemporalAA" 1e+02 5e+01 0.6 (Utilities|Array|MakeArray 0)))
              ;[1 1 1] Draw Inventory
              (if (Variables|Default|GetInventoryOpen)
                (Variables|/Script/Engine.SpringArmComponent|SetTargetArmLength (Variables|/Game/Blueprints/PlayerCharacter.PlayerCharacter_C|GetSpringArm1 _asplayercharacter_c) 4.5e+02)
                (if (Math|Conversions|ToBoolean(Integer) (Utilities|Array|Length (Variables|Default|GetInventoryPositions)))
                  _
                  (else
                    (CallFunction|CalculateInventoryPositions)))
                (CallFunction|AddHitboxes)
                (bind (_transparency _secondtransparency) (CallFunction|CalculateTransparency _x _y))
                (HUD|DrawRect (Math|Color|MakeColor 1.0 1.0 1.0 _transparency) (- _x 1e+01) (- _y 1e+01) 2e+01 2e+01)
                (CallFunction|DrawBox (Utilities|Array|Get(acopy) (Variables|Default|GetItemboxes)) _secondtransparency)
                (bind _transparency_2 (CallFunction|CalculateTransparency _x_3 _y_3))
                (HUD|DrawRect (Math|Color|MakeColor 1.0 1.0 1.0 _transparency_2) (- _x_3 1e+01) (- _y_3 1e+01) 2e+01 2e+01)
                (bind _transparency_3 (CallFunction|CalculateTransparency _x_4 _y_4))
                (HUD|DrawRect (Math|Color|MakeColor 1.0 1.0 1.0 _transparency_3) (- _x_4 1e+01) (- _y_4 1e+01) 2e+01 2e+01)
                (bind _transparency_4 (CallFunction|CalculateTransparency _x_2 _y_2))
                (HUD|DrawRect (Math|Color|MakeColor 1.0 1.0 1.0 _transparency_4) (- _x_2 1e+01) (- _y_2 1e+01) 2e+01 2e+01)
                (else
                  (Variables|/Script/Engine.SpringArmComponent|SetTargetArmLength (Variables|/Game/Blueprints/PlayerCharacter.PlayerCharacter_C|GetSpringArm1 _asplayercharacter_c) 6e+02))))))))
    (:then_2
      (HUD|DrawText (Utilities|String|Append "Kills: " (Utilities|String|ToString(Integer) (Variables|Default|GetKillCount))) "(R=1.000000,G=1.000000,B=1.000000,A=1.000000)" 1e+01 1e+01 "/Game/Fonts/StandardFont.StandardFont" 1.5 false))))

(event EventHitBoxEndCursorOver
  (params (BoxName :type Name :default "None"))
  (bind _itemboxes (Variables|Default|GetItemboxes))
  (bind _itembuttons (Variables|Default|GetItemButtons))
  ;[1 1 1] Draw Inventory
  (for (_array_element _array_index) _itemboxes
    (if (Utilities|Name|Equal(Name) (.HitboxName (Utilities|Struct|BreakScrollbox _array_element)) BoxName)
      (Utilities|Array|SetArrayElem _itemboxes _array_index (Utilities|Struct|MakeScrollbox false (.Buttons (Utilities|Struct|BreakScrollbox _array_element)) (.HitboxName (Utilities|Struct|BreakScrollbox _array_element)) (.Position (Utilities|Struct|BreakScrollbox _array_element))))))
  (for (_array_element_2 _array_index_2) _itembuttons
    (if (Utilities|Name|Equal(Name) (.HitboxName (Utilities|Struct|BreakItemButton _array_element_2)) BoxName)
      (Utilities|Array|SetArrayElem _itembuttons _array_index_2 (Utilities|Struct|MakeItemButton false (.Equipped (Utilities|Struct|BreakItemButton _array_element_2)) (.Icon (Utilities|Struct|BreakItemButton _array_element_2)) (.HitboxName (Utilities|Struct|BreakItemButton _array_element_2)) (.ItemClass (Utilities|Struct|BreakItemButton _array_element_2)) (.Position (Utilities|Struct|BreakItemButton _array_element_2)))))))

(event EventHitBoxBeginCursorOver
  (params (BoxName :type Name :default "None"))
  (bind _itemboxes (Variables|Default|GetItemboxes))
  (bind _itembuttons (Variables|Default|GetItemButtons))
  ;[1 1 1] Draw Inventory
  (for (_array_element _array_index) _itemboxes
    (if (Utilities|Name|Equal(Name) (.HitboxName (Utilities|Struct|BreakScrollbox _array_element)) BoxName)
      (Utilities|Array|SetArrayElem _itemboxes _array_index (Utilities|Struct|MakeScrollbox true (.Buttons (Utilities|Struct|BreakScrollbox _array_element)) (.HitboxName (Utilities|Struct|BreakScrollbox _array_element)) (.Position (Utilities|Struct|BreakScrollbox _array_element))))))
  (for (_array_element_2 _array_index_2) _itembuttons
    (if (Utilities|Name|Equal(Name) (.HitboxName (Utilities|Struct|BreakItemButton _array_element_2)) BoxName)
      (Utilities|Array|SetArrayElem _itembuttons _array_index_2 (Utilities|Struct|MakeItemButton true (.Equipped (Utilities|Struct|BreakItemButton _array_element_2)) (.Icon (Utilities|Struct|BreakItemButton _array_element_2)) (.HitboxName (Utilities|Struct|BreakItemButton _array_element_2)) (.ItemClass (Utilities|Struct|BreakItemButton _array_element_2)) (.Position (Utilities|Struct|BreakItemButton _array_element_2)))))))

(event Input|MouseEvents|MouseWheelUp
  ;[1 1 1] Draw Inventory
  (:Pressed
    (for _array_element (Variables|Default|GetItemboxes)
      (if (.Active (Utilities|Struct|BreakScrollbox _array_element))
        (CallFunction|Scroll true _array_element)))))

(event Input|MouseEvents|MouseWheelDown
  ;[1 1 1] Draw Inventory
  (:Pressed
    (for _array_element (Variables|Default|GetItemboxes)
      (if (.Active (Utilities|Struct|BreakScrollbox _array_element))
        (CallFunction|Scroll false _array_element)))))

(fn ConstructionScript)

(fn CalculateTransparency
  (params (XPos :type Float%20%28single-precision%29) (YPos :type Float%20%28single-precision%29))
  (bind _returnvalue (Game|GetPlayerCharacter 0))
  (bind _returnvalue_2 (Game|GetPlayerController 0))
  (bind (_locationx _locationy) (Game|Player|GetMousePosition _returnvalue_2))
  (bind _returnvalue_3 (Transformation|GetActorLocation _returnvalue))
  (bind _returnvalue_4 (Class|HUD|Project _returnvalue_3))
  (bind (_x _y) (Math|Vector|BreakVector _returnvalue_4))
  (bind _returnvalue_5 (- XPos _x))
  (bind _returnvalue_6 (- YPos _y))
  (bind _returnvalue_7 (- _locationy _y))
  (bind _returnvalue_8 (- _locationx _x))
  (bind _returnvalue_9 (Math|Vector|MakeVector 0.0 _returnvalue_8 _returnvalue_7))
  (bind _returnvalue_10 (Math|Vector|MakeVector 0.0 _returnvalue_5 _returnvalue_6))
  (bind _returnvalue_11 (Math|Vector|Normalize _returnvalue_9))
  (bind _returnvalue_12 (Math|Vector|Normalize _returnvalue_10))
  (bind _returnvalue_13 (Math|Vector|VectorLength _returnvalue_9))
  (bind _returnvalue_14 (Math|Vector|DotProduct _returnvalue_11 _returnvalue_12))
  (return (Math|Float|Clamp(Float) (* (Math|Float|Clamp(Float) (/ _returnvalue_13 1e+02)) _returnvalue_14) 0.3) (Math|Float|Clamp(Float) (* (Math|Float|Clamp(Float) (/ _returnvalue_13 2e+02)) _returnvalue_14))))

(fn OpenInventory
  (Variables|Default|SetInventoryOpen true)
  (Utilities|Array|Clear (Variables|Default|GetInventoryPositions))
  (Input|EnableInput (Game|GetPlayerController 0)))

(fn CloseInventory
  (Variables|Default|SetInventoryOpen false)
  (Input|DisableInput (Game|GetPlayerController 0)))

(fn CalculateInventoryPositions
  (bind _returnvalue (Game|GetPlayerCharacter 0))
  (bind _inventorypositions (Variables|Default|GetInventoryPositions))
  (bind _returnvalue_2 (Transformation|GetActorLocation _returnvalue))
  (bind _returnvalue_3 (Class|HUD|Project _returnvalue_2))
  (bind (_x _y) (Math|Vector|BreakVector _returnvalue_3))
  (bind _returnvalue_4 (- _x 1.5e+02))
  (bind _returnvalue_5 (Math|Vector2D|MakeVector2D _returnvalue_4 _y))
  (Utilities|Array|Add _inventorypositions _returnvalue_5)
  (Utilities|Array|Add _inventorypositions (Math|Vector2D|MakeVector2D (+ _x 1.5e+02) _y))
  (Utilities|Array|Add _inventorypositions (Math|Vector2D|MakeVector2D _x (- _y 1.5e+02)))
  (Utilities|Array|Add _inventorypositions (Math|Vector2D|MakeVector2D _x (+ _y 1.5e+02)))
  (Utilities|Array|Add (Variables|Default|GetItemboxes) (Utilities|Struct|MakeScrollbox false (Utilities|Array|MakeArray) "W" (- _returnvalue_5 "(X=250.000000,Y=112.000000)")))
  (for _index (range 0 12)
    (CallFunction|AddButton (Utilities|Array|Get(acopy) (Variables|Default|GetItemboxes)) "/Game/Blueprints/Items/BaseItem.BaseItem_C")))

(fn Scroll
  (params (Up :type Boolean) (Box :type Scrollbox%20Structure%20%28by%20ref%29))
  (bind (_active _buttons _hitboxname _position) (Utilities|Struct|BreakScrollbox Box))
  (bind _itembuttons (Variables|Default|GetItemButtons))
  (bind _buttons_2 (LocalVariables|Getbuttons))
  (for _array_element _itembuttons
    (if (Utilities|Enum|Equal(Enum) (Utilities|String|GetSubstring (Utilities|String|ToString(Name) (.HitboxName (Utilities|Struct|BreakItemButton _array_element))) 0) (Utilities|String|ToString(Name) _hitboxname))
      (Utilities|Array|Add (LocalVariables|Getbuttons) _array_element)))
  (if (> (Utilities|Array|Length _buttons_2) 9)
    (if (or (and Up (< (.Y (Math|Vector2D|BreakVector2D (.Position (Utilities|Struct|BreakItemButton (Utilities|Array|Get(acopy) _buttons_2))))) (.Y (Math|Vector2D|BreakVector2D _position)))) (and (not Up) (> (.Y (Math|Vector2D|BreakVector2D (.Position (Utilities|Struct|BreakItemButton (Utilities|Array|Get(acopy) _buttons_2 (Utilities|Array|LastIndex _buttons_2)))))) (+ (.Y (Math|Vector2D|BreakVector2D _position)) 224.0))))
      (for _array_element_2 _buttons_2
        (Utilities|Array|SetArrayElem _itembuttons (Utilities|Array|FindItem _buttons_2 _array_element_2) (Utilities|Struct|MakeItemButton (.MouseOver (Utilities|Struct|BreakItemButton _array_element_2)) (.Equipped (Utilities|Struct|BreakItemButton _array_element_2)) (.Icon (Utilities|Struct|BreakItemButton _array_element_2)) (.HitboxName (Utilities|Struct|BreakItemButton _array_element_2)) (.ItemClass (Utilities|Struct|BreakItemButton _array_element_2)) (+ (.Position (Utilities|Struct|BreakItemButton _array_element_2)) (Math|Vector2D|MakeVector2D 0.0 (Math|Float|SelectFloat 8e+01 -8e+01 Up)))))))))

(fn DrawBox
  (params (Box :type Scrollbox%20Structure) (Transparency :type Float%20%28single-precision%29))
  (bind (_active _buttons _hitboxname _position) (Utilities|Struct|BreakScrollbox Box))
  (bind _y (Math|Vector2D|BreakVector2D _position))
  (for _array_element (Variables|Default|GetItemButtons)
    (if (Utilities|Enum|Equal(Enum) (Utilities|String|GetSubstring (Utilities|String|ToString(Name) (.HitboxName (Utilities|Struct|BreakItemButton _array_element))) 0) (Utilities|String|ToString(Name) _hitboxname))
      (if (and (>= (.Y (Math|Vector2D|BreakVector2D (.Position (Utilities|Struct|BreakItemButton _array_element)))) _y) (< (.Y (Math|Vector2D|BreakVector2D (.Position (Utilities|Struct|BreakItemButton _array_element)))) (+ _y 224.0)))
        (Canvas|DrawTexture (.Icon (Utilities|Struct|BreakItemButton _array_element)) (.X (Math|Vector2D|BreakVector2D (.Position (Utilities|Struct|BreakItemButton _array_element)))) (.Y (Math|Vector2D|BreakVector2D (.Position (Utilities|Struct|BreakItemButton _array_element)))) 128.0 128.0 0.0 0.0 1.0 1.0 (Math|Color|SelectColor (Math|Color|MakeColor 1.0 1.0 1.0 Transparency) (Math|Color|MakeColor 1.0 1.0 1.0 (/ Transparency 2.0)) (.MouseOver (Utilities|Struct|BreakItemButton _array_element))) "BLEND_Translucent" 0.5)))))

(fn AddHitboxes
  (for _array_element (Variables|Default|GetItemboxes)
    (Class|HUD|AddHitBox (.Position (Utilities|Struct|BreakScrollbox _array_element)) "(X=224.000000,Y=224.000000)" (.HitboxName (Utilities|Struct|BreakScrollbox _array_element)) false))
  (for _array_element_2 (Variables|Default|GetItemButtons)
    (Class|HUD|AddHitBox (.Position (Utilities|Struct|BreakItemButton _array_element_2)) "(X=64.000000,Y=64.000000)" (.HitboxName (Utilities|Struct|BreakItemButton _array_element_2)) false)))

(fn AddButton
  (params (Box :type Scrollbox%20Structure%20%28by%20ref%29) (Item :type Base%20Item%20Class%20Reference))
  (bind (_active _buttons _hitboxname _position) (Utilities|Struct|BreakScrollbox Box))
  (bind _itembuttons (Variables|Default|GetItemButtons))
  (bind _buttons_2 (LocalVariables|Getbuttons))
  (bind _returnvalue (Utilities|Array|Length _buttons_2))
  (bind _returnvalue_2 (Utilities|String|ToString(Name) _hitboxname))
  (bind _returnvalue_3 (Utilities|String|ToString(Integer) _returnvalue))
  (bind _returnvalue_4 (Math|Integer|%(Integer) _returnvalue 3))
  (bind _returnvalue_5 (== _returnvalue_4 0))
  (bind _returnvalue_6 (Utilities|String|Append _returnvalue_2 _returnvalue_3))
  (bind _returnvalue_7 (Utilities|String|StringToName _returnvalue_6))
  (for _array_element (Variables|Default|GetItemButtons)
    (if (Utilities|Enum|Equal(Enum) (Utilities|String|GetSubstring (Utilities|String|ToString(Name) (.HitboxName (Utilities|Struct|BreakItemButton _array_element))) 0) (Utilities|String|ToString(Name) _hitboxname))
      (Utilities|Array|Add (LocalVariables|Getbuttons) _array_element)))
  (if (== _returnvalue 0)
    (Utilities|Array|Add _itembuttons (Utilities|Struct|MakeItemButton false false "/Game/Blueprints/Testicon.Testicon" _returnvalue_7 Item _position))
    (else
      (Utilities|Array|Add _itembuttons (Utilities|Struct|MakeItemButton false false "/Game/Blueprints/Testicon.Testicon" _returnvalue_7 Item (+ (.Position (Utilities|Struct|BreakItemButton (Utilities|Array|Get(acopy) _itembuttons (- (Utilities|Array|Length _itembuttons) 1)))) (Math|Vector2D|MakeVector2D (Math|Float|SelectFloat -1.6e+02 8e+01 _returnvalue_5) (Math|Float|SelectFloat 8e+01 0.0 _returnvalue_5))))))))