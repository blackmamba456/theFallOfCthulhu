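; BP_LevelExit is a level exit actor that advances the game to the next level.
; When the player pawn begins overlapping it, it binds its ExitLevel event to an event dispatcher on PlayerCharacter.
; ExitLevel calls NextLevel on the MyGame game mode.
; End overlap makes the same bind call rather than an unbind, so leaving the area does not remove the binding.
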(event `self.ReceiveActorBeginOverlap`
  (params (OtherActor :type "Actor Object Reference"))
  (bind _returnvalue (`GameplayStatics.GetPlayerPawn` 0))
  (if (== _returnvalue OtherActor)
    (bind _asplayercharacter_c (cast `/Game/Blueprints/PlayerCharacter` _returnvalue))
    (add `/Game/Blueprints/PlayerCharacter.ActionDispatcher` _asplayercharacter_c (delegate `ExitLevel`))))

(event `ExitLevel`
  (bind _asmygame_c (cast `/Game/Blueprints/Game/MyGame` (`GameplayStatics.GetGameMode`)))
  (`/Game/Blueprints/Game/MyGame.NextLevel` _asmygame_c))

(event `self.ReceiveActorEndOverlap`
  (params (OtherActor :type "Actor Object Reference"))
  (bind _returnvalue (`GameplayStatics.GetPlayerPawn` 0))
  (if (== _returnvalue OtherActor)
    (bind _asplayercharacter_c (cast `/Game/Blueprints/PlayerCharacter` _returnvalue))
    (add `/Game/Blueprints/PlayerCharacter.ActionDispatcher` _asplayercharacter_c (delegate `ExitLevel`))))

(fn `UserConstructionScript`)